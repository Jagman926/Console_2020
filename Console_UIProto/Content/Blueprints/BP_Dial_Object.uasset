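; BP_Dial_Object is a rotatable dial actor that spawns a BP_PushDial_UI at its root on BeginPlay and hands it a self-reference.
; Start and Stop events bracket a rotation, recording the starting rolls of the dial and the driving input.
; While active, RotateDial applies the input's change since start to the dial's roll, wrapped to 0-360, preserving pitch and yaw and storing DialRoll.
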(event `self.ReceiveBeginPlay`
  (bind _returnvalue (`|SpawnActorFromClass` "/Game/Blueprints/BP_PushDial_UI.BP_PushDial_UI_C" (`KismetMathLibrary.MakeTransform` (`SceneComponent.K2_GetComponentLocation` (`self.DefaultSceneRoot`)) (struct :`Yaw` 180.0)) "Undefined" "OverrideRootScale" null null))
  (set `/Game/Blueprints/BP_PushDial_UI.dial_Object` self _returnvalue))

(event `self.ReceiveTick`
  (params (DeltaSeconds :type "Float (single-precision)")))

(event `Rotate Dial`
  (params (`Relative Roll` :type "Float (double-precision)"))
  (if (`self.dialIsRotating`)
    (bind _newrotation (`self.AddRollRotationByDifference` `Relative Roll` (`self.thisRollStart`) (`self.otherRollStart`)))
    (`self.K2_SetActorRotation` _newrotation)
    (set `self.dialRoll` (.roll _newrotation))))

(event `Start Dial Rotation`
  (params (startingRollRotation :type "Float (double-precision)"))
  (set `self.otherRollStart` startingRollRotation)
  (set `self.thisRollStart` (.roll (`self.K2_GetActorRotation` self)))
  (set `self.dialIsRotating` true))

(event `Stop Dial Rotation`
  (set `self.otherRollStart` 0.0)
  (set `self.thisRollStart` 0.0)
  (set `self.dialIsRotating` false))

(fn `AddRollRotationByDifference`
  (params (rollAdditive :type "Float (double-precision)") (thisRollStart :type "Float (double-precision)") (otherRollStart :type "Float (double-precision)"))
  (returns (newRotation :type "Rotator Structure"))
  (bind _out (`self.RadialClamp` (- (+ rollAdditive thisRollStart) otherRollStart))) ; Clamps to 0-360
  (return (`KismetMathLibrary.MakeRotator` _out (.pitch (`self.K2_GetActorRotation` self)) (.yaw (`self.K2_GetActorRotation` self)))))

(fn `RadialClamp`
  (params (degree :type "Float (double-precision)"))
  (returns (out :type "Float (double-precision)"))
  (bind _returnvalue (mod degree 360.0))
  (if (< degree 0.0)
    (return (+ _returnvalue 360.0))
    (else
      (return _returnvalue))))

(fn `UserConstructionScript`)