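; VR push dial actor that rotates to pick a stepped integer value and presses in to toggle between Set and Unset.
; Externally driven rotation events apply hand-roll difference, snapping to increments with haptic and sound ticks.
; On Tick, the closest overlapping motion controller's distance lerps dial and value widget along world X, flipping state at bottom-out.
; The widget shows value and state color; BeginPlay also spawns a linked BP_PushDial_UI.
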(event `Update Dial UI Value`
  (params (dialValue :type Integer))
  ;[1 0.8357 0.1739] UI Update Functions
  (bind _asuiw_variable (cast `/Game/UIAssets/UIW_Variable` (`WidgetComponent.GetUserWidgetObject` (`self.variableUIW`))))
  (`/Game/UIAssets/UIW_Variable.Update Variable` _asuiw_variable (`KismetTextLibrary.Conv_IntToText` dialValue)))

(event `self.ReceiveBeginPlay`
  (`self.InitPushDialMinMax`)
  (bind _returnvalue (`|SpawnActorFromClass` "/Game/Blueprints/PushDial/BP_PushDial_UI.BP_PushDial_UI_C" (`KismetMathLibrary.MakeTransform` (`SceneComponent.K2_GetComponentLocation` (`self.DefaultSceneRoot`)) (struct :`Yaw` 180.0)) "Undefined" "OverrideRootScale" null null))
  (set `/Game/Blueprints/PushDial/BP_PushDial_UI.dial_Object` self _returnvalue)
  (set `self.rotationIncrementBy360` (/ 360.0 (`self.rotationMax`)))
  (bind _output_get (set `self.dialState` "NewEnumerator3"))
  (`self.Update Dial UI Color By State` _output_get))

(event `Update Dial UI Color`
  (params (color :type "LinearColor Structure"))
  ;[1 0.8357 0.1739] UI Update Functions
  (bind _asuiw_variable (cast `/Game/UIAssets/UIW_Variable` (`WidgetComponent.GetUserWidgetObject` (`self.variableUIW`))))
  (`/Game/UIAssets/UIW_Variable.Update Color` _asuiw_variable color))

(event `self.ReceiveTick`
  (params (DeltaSeconds :type "Float (single-precision)"))
  (bind _ispushing (`self.CheckIfPushingDial`))
  (if _ispushing
    (`self.Push Dial`)
    (else
      (`self.Reset Dial and UI Location`))))

(event `Update Dial UI Color By State`
  (params (dialState :type "/Game/Enums/dialState Enum" :default "NewEnumerator0"))
  ;[1 0.8357 0.1739] UI Update Functions
  (switch `/Game/Enums/dialState` dialState
    (:`NewEnumerator0`
      (`self.Update Dial UI Color` (struct :`A` 1.0)))
    (:`NewEnumerator1`
      (`self.Update Dial UI Color` (struct :`R` 0.054902 :`G` 0.686275 :`B` 1.0 :`A` 1.0)))
    (:`NewEnumerator2`
      (`self.Update Dial UI Color` (struct :`R` 0.164706 :`G` 1.0 :`B` 0.262745 :`A` 1.0)))
    (:`NewEnumerator3`
      (`self.Update Dial UI Color` (struct :`R` 1.0 :`G` 0.247059 :`B` 0.278431 :`A` 1.0)))))

(event `Rotate Dial`
  (params (`Relative Roll` :type "Float (double-precision)"))
  ;[0.4503 0.7522 1] Rotate Dial Functions
  (if (`self.dialIsRotating`)
    (bind _newrotation (`self.AddRollRotationByDifference` `Relative Roll` (`self.thisRollStart`) (`self.otherRollStart`)))
    (bind _output_get (set `self.dialRoll` (.roll _newrotation)))
    (bind _dialvalue (`self.SetDialValueByRoll` _output_get))
    (`self.Update Dial UI Value` _dialvalue)
    (bind _dialroll (`self.SetDialRollByValue` _dialvalue))
    (`self.K2_SetActorRotation` (`KismetMathLibrary.MakeRotator` _dialroll (.pitch _newrotation) (.yaw _newrotation)))
    (`SceneComponent.K2_SetWorldTransform` (`self.variableUIW`) (`self.variableUIWStartTransform`) false false)))

(event `Start Dial Rotation`
  (params (startingRollRotation :type "Float (double-precision)"))
  ;[0.4503 0.7522 1] Rotate Dial Functions
  (set `self.otherRollStart` startingRollRotation)
  (set `self.thisRollStart` (.roll (`self.K2_GetActorRotation` self)))
  (set `self.dialIsRotating` true)
  (bind _output_get (set `self.dialState` "NewEnumerator1"))
  (`self.Update Dial UI Color By State` _output_get))

(event `Reset Dial and UI Location`
  (bind _dialstate (`self.dialState`))
  (bind _pushdial_starttransform_location (`KismetMathLibrary.BreakTransform` (`self.PushDial_StartTransform`)))
  (bind _pushdial_setpushtransform_location (`KismetMathLibrary.BreakTransform` (`self.PushDial_SetPushTransform`)))
  (bind _variableuiwsetpushtransform_location (`KismetMathLibrary.BreakTransform` (`self.variableUIWSetPushTransform`)))
  (bind _variableuiwstarttransform_location (`KismetMathLibrary.BreakTransform` (`self.variableUIWStartTransform`)))
  ;[1 0.4305 0.2598] Dial Update Functions
  (if (or (`|EnumEquality` _dialstate "NewEnumerator3") (`|EnumEquality` _dialstate "NewEnumerator1"))
    (`self.SetPushDialAndUILocation` _pushdial_starttransform_location _variableuiwstarttransform_location)
    (else
      (`self.SetPushDialAndUILocation` _pushdial_setpushtransform_location _variableuiwsetpushtransform_location))))

(event `Stop Dial Rotation`
  ;[0.4503 0.7522 1] Rotate Dial Functions
  (set `self.otherRollStart` 0.0)
  (set `self.thisRollStart` 0.0)
  (set `self.dialIsRotating` false)
  (bind _output_get (set `self.dialState` "NewEnumerator3"))
  (`self.Update Dial UI Color By State` _output_get))

(event `Update Grabbing Hand`
  (params (grabbingHand :type "SceneComponent Object Reference"))
  ;[1 0.4305 0.2598] Dial Update Functions
  (set `self.grabbingHand` grabbingHand))

(event `Push Dial`
  (bind _pushdial_starttransform_location (`KismetMathLibrary.BreakTransform` (`self.PushDial_StartTransform`)))
  (bind _pushdial_endpushtransform_location (`KismetMathLibrary.BreakTransform` (`self.PushDial_EndPushTransform`)))
  (bind _variableuiwstarttransform_location (`KismetMathLibrary.BreakTransform` (`self.variableUIWStartTransform`)))
  (bind _variableuiwendpushtransform_location (`KismetMathLibrary.BreakTransform` (`self.variableUIWEndPushTransform`)))
  ;[1 0.4618 0.8866] Push Dial Functions
  (bind _alpha (`self.GetUnsetPushAlpha`)) ; Alpha between  0 and 1 (1 being pushed completely in)
  (`self.SetPushDialAndUILocation` (`KismetMathLibrary.VLerp` _pushdial_starttransform_location _pushdial_endpushtransform_location _alpha) (`KismetMathLibrary.VLerp` _variableuiwstarttransform_location _variableuiwendpushtransform_location _alpha)) ; Applies lerped location value to dial location
  (if (> _alpha (+ (/ (`self.SetAmount_xAxis`) 10.0) (/ (`self.ClickAmountOffset_xAxis`) 10.0)))
    ;;[1 1 1] Dial State Switch when hitting bottom out
    (`/Engine/EditorBlueprintResources/StandardMacros.DoOnce` false :!label _label
      (:`Completed`
        (`self.Click Switch State`)
        (`GameplayStatics.PlaySound2D` "/Game/Audio/Tick.Tick" 1.0 0.8 0.0 null null)
        (goto _label_2 :!via `Reset`)))
    (else
      (`/Engine/EditorBlueprintResources/StandardMacros.DoOnce` true :!label _label_2
        (:`Completed`
          (`GameplayStatics.PlaySound2D` "/Game/Audio/Tick.Tick" 1.0 0.65 0.0 null null)
          (goto _label :!via `Reset`))))))

(event `Start Dial Push`
  ;[1 0.4618 0.8866] Push Dial Functions
  (set `self.isPushing` true))

(event `Stop Dial Push`
  ;[1 0.4618 0.8866] Push Dial Functions
  (set `self.isPushing` false)
  (`self.Reset Dial and UI Location`) ; resets dial ui position to OnBegin values
)

(event `Click Switch State`
  ;[1 0.4618 0.8866] Push Dial Functions
  (if (`|EnumEquality` (`self.dialState`) "NewEnumerator2")
    (set `self.dialState` "NewEnumerator3")
    (else
      (set `self.dialState` "NewEnumerator2")))
  (`self.Update Dial UI Color By State` (`self.dialState`)))

(event `self.Dial.OnComponentBeginOverlap`
  (params (OverlappedComponent :type "PrimitiveComponent Object Reference") (OtherActor :type "Actor Object Reference") (OtherComp :type "PrimitiveComponent Object Reference") (OtherBodyIndex :type Integer) (bFromSweep :type Boolean) (SweepResult :type "HitResult Structure (by ref)"))
  (bind _overlappinghandarray (`self.overlappingHandArray`))
  ;[0.4858 1 0.4688] Dial Overlap Begin / End
  (bind _asbp_motion_controller (cast `/Game/VirtualRealityBP/Blueprints/BP_MotionController` OtherActor))
  (if (== (`self.numberOfHandOverlaps`) 0)
    (`self.Start Dial Push`))
  (`/Engine/EditorBlueprintResources/StandardMacros.IncrementInt` (`self.numberOfHandOverlaps`)
    (:`  `
      ;;[1 1 1] Adds hand to array of overlapping hands
      (`KismetArrayLibrary.Array_Add` _overlappinghandarray _asbp_motion_controller)
      (set `self.numberOfHandOverlaps` (`KismetArrayLibrary.Array_Length` _overlappinghandarray)))))

(event `self.Dial.OnComponentEndOverlap`
  (params (OverlappedComponent :type "PrimitiveComponent Object Reference") (OtherActor :type "Actor Object Reference") (OtherComp :type "PrimitiveComponent Object Reference") (OtherBodyIndex :type Integer))
  (bind _overlappinghandarray (`self.overlappingHandArray`))
  ;[0.4858 1 0.4688] Dial Overlap Begin / End
  (bind _asbp_motion_controller (cast `/Game/VirtualRealityBP/Blueprints/BP_MotionController` OtherActor))
  (bind _result (`/Engine/EditorBlueprintResources/StandardMacros.DecrementInt` (`self.numberOfHandOverlaps`))
    (:`  `
      (if (== _result 0)
        (`self.Stop Dial Push`))
      ;;[1 1 1] Removes hand for overlapping hand array
      (`KismetArrayLibrary.Array_RemoveItem` _overlappinghandarray _asbp_motion_controller)
      (set `self.numberOfHandOverlaps` (`KismetArrayLibrary.Array_Length` _overlappinghandarray)))))

(fn `AddRollRotationByDifference`
  (params (rollAdditive :type "Float (double-precision)") (thisRollStart :type "Float (double-precision)") (otherRollStart :type "Float (double-precision)"))
  (returns (newRotation :type "Rotator Structure"))
  (bind _out (`self.RadialClamp` (- (+ rollAdditive thisRollStart) otherRollStart))) ; Clamps to 0-360
  (return (`KismetMathLibrary.MakeRotator` _out (.pitch (`self.K2_GetActorRotation` self)) (.yaw (`self.K2_GetActorRotation` self)))))

(fn `CheckIfPushingDial`
  (returns (isPushing :type Boolean))
  (if (and (`self.isPushing`) (`|EnumInequality` (`self.dialState`) "NewEnumerator1"))
    (bind (_hand _distance_from_dial) (`self.GetClosestOverlappingHand` (`self.overlappingHandArray`)))
    (if (`|EnumInequality` (`self.dialState`) "NewEnumerator2")
      (return (and (`KismetSystemLibrary.IsValid` _hand) (< _distance_from_dial (`self.minimumDistanceFromDial`))))
      (else
        (return (and (`KismetSystemLibrary.IsValid` _hand) (< _distance_from_dial (- (`self.minimumDistanceFromDial`) (`self.SetAmount_xAxis`)))))))
    (else
      (return false))))

(fn `GetClosestOverlappingHand`
  (params (overlappingHands :type "Array of /Game/VirtualRealityBP/Blueprints/BP_MotionController Object Reference"))
  (returns (hand :type "/Game/VirtualRealityBP/Blueprints/BP_MotionController Object Reference") (`Distance From Dial` :type "Float (double-precision)"))
  (locals (closestHand :type "/Game/VirtualRealityBP/Blueprints/BP_MotionController Object Reference") (closestHandDistance :type "Float (double-precision)" :default 100000000.0))
  (if (> (`KismetArrayLibrary.Array_Length` overlappingHands) 0)
    (for _array_element overlappingHands
      (bind _returnvalue (`KismetMathLibrary.Vector_Distance` (`SceneComponent.K2_GetComponentLocation` (`/Game/VirtualRealityBP/Blueprints/BP_MotionController.GrabSphere` _array_element)) (`SceneComponent.K2_GetComponentLocation` (`self.Dial`))))
      (if (< _returnvalue (`local.closestHandDistance`))
        (set `local.closestHand` _array_element)
        (set `local.closestHandDistance` _returnvalue)))
    (return (`local.closestHand`) (`local.closestHandDistance`))
    (else
      (`KismetSystemLibrary.PrintString` "GetClosestOverlappingHand: Hand Array is Empty" true true (struct :`R` 1.0 :`B` 0.024906 :`A` 1.0) 10.0)
      (return null -1.0))))

(fn `GetUnsetPushAlpha`
  (returns (alpha :type "Float (double-precision)"))
  (bind _minimumdistancefromdial (`self.minimumDistanceFromDial`))
  (bind (_hand _distance_from_dial) (`self.GetClosestOverlappingHand` (`self.overlappingHandArray`)))
  (if (< _distance_from_dial _minimumdistancefromdial)
    (return (`KismetMathLibrary.NormalizeToRange` (- _minimumdistancefromdial _distance_from_dial) 0.0 _minimumdistancefromdial))))

(fn `InitPushDialMinMax`
  (bind _output_get (set `self.variableUIWStartTransform` (`SceneComponent.K2_GetComponentToWorld` (`self.variableUIW`))))
  (set `self.variableUIWEndPushTransform` (`KismetMathLibrary.MakeTransform` (`KismetMathLibrary.MakeVector` (+ (.x (.location _output_get)) (`self.PushAmount_xAxis`)) (.y (.location _output_get)) (.z (.location _output_get))) (.rotation _output_get) (.scale _output_get)))
  (set `self.variableUIWSetPushTransform` (`KismetMathLibrary.MakeTransform` (`KismetMathLibrary.MakeVector` (+ (.x (.location _output_get)) (`self.SetAmount_xAxis`)) (.y (.location _output_get)) (.z (.location _output_get))) (.rotation _output_get) (.scale _output_get)))
  (bind _output_get_2 (set `self.PushDial_StartTransform` (`SceneComponent.K2_GetComponentToWorld` (`self.Dial`))))
  (set `self.PushDial_EndPushTransform` (`KismetMathLibrary.MakeTransform` (`KismetMathLibrary.MakeVector` (+ (.x (.location _output_get_2)) (`self.PushAmount_xAxis`)) (.y (.location _output_get_2)) (.z (.location _output_get_2))) (.rotation _output_get_2) (.scale _output_get_2)))
  (set `self.PushDial_SetPushTransform` (`KismetMathLibrary.MakeTransform` (`KismetMathLibrary.MakeVector` (+ (.x (.location _output_get_2)) (`self.SetAmount_xAxis`)) (.y (.location _output_get_2)) (.z (.location _output_get_2))) (.rotation _output_get_2) (.scale _output_get_2))))

(fn `PushBottomOutFeedback`
  (params (pushingHand :type "SceneComponent Object Reference"))
  (bind _asmotion_controller_component (cast `MotionControllerComponent` pushingHand))
  (bind _returnvalue (`MagicLeapControllerFunctionLibrary.GetHandForMotionSource` (`MotionControllerComponent.MotionSource` _asmotion_controller_component)))
  (`PlayerController.PlayHapticEffect` (`GameplayStatics.GetPlayerController` 0) "/Game/HapticFeedback/BottomOut_HapticFeedbackEffect_Curve.BottomOut_HapticFeedbackEffect_Curve" _returnvalue 1.0 false))

(fn `RadialClamp`
  (params (degree :type "Float (double-precision)"))
  (returns (out :type "Float (double-precision)"))
  (bind _returnvalue (mod degree 360.0))
  (if (< degree 0.0)
    (return (+ _returnvalue 360.0))
    (else
      (return _returnvalue))))

(fn `SetDialRollByValue`
  (params (dialValue :type Integer))
  (returns (dialRoll :type "Float (double-precision)"))
  (bind _output_get (set `self.dialRoll` (* dialValue (`self.rotationIncrementBy360`))))
  (return _output_get))

(fn `SetDialValueByRoll`
  (params (roll :type "Float (double-precision)"))
  (returns (dialValue :type Integer))
  (bind (_remainder _returnvalue) (`KismetMathLibrary.FMod` roll (`self.rotationIncrementBy360`)))
  (if (!= _returnvalue (`self.dialValue`))
    (`self.TickFeedback` (`self.grabbingHand`)))
  (bind _output_get (set `self.dialValue` _returnvalue))
  (return _output_get))

(fn `SetPushDialAndUILocation`
  (params (pushDialLocation :type "Vector Structure") (uiLocation :type "Vector Structure"))
  (`SceneComponent.K2_SetWorldLocation` (`self.Dial`) pushDialLocation false false)
  (`SceneComponent.K2_SetWorldLocation` (`self.variableUIW`) uiLocation false false))

(fn `TickFeedback`
  (params (grabbingHand :type "SceneComponent Object Reference"))
  (bind _asmotion_controller_component (cast `MotionControllerComponent` grabbingHand))
  (bind _returnvalue (`MagicLeapControllerFunctionLibrary.GetHandForMotionSource` (`MotionControllerComponent.MotionSource` _asmotion_controller_component)))
  (`PlayerController.PlayHapticEffect` (`GameplayStatics.GetPlayerController` 0) "/Game/VirtualRealityBP/Blueprints/MotionControllerHaptics.MotionControllerHaptics" _returnvalue 1.0 false)
  (`GameplayStatics.PlaySound2D` "/Game/Audio/Tick.Tick" 0.5 1.0 0.0 null null))

(fn `UserConstructionScript`)