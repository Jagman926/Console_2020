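; BP_Pickup_Cube_UI is a child of BP_Pickup_Cube, a pickup cube that, judging by its name, serves as a UI variant.
; Its Pickup and Drop events only call the parent implementations, and its construction script does the same.
; BeginPlay, overlap and Tick are disabled placeholder nodes, so the graphs add no behavior of their own.
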(event `/Game/VirtualRealityBP/Blueprints/PickupActorInterface.Pickup`
  (params (AttachTo :type "SceneComponent Object Reference"))
  ;[0.402 0.7758 1] Calls parent BP_Pickup_Cube Pickup functionality
  (`parent.Pickup` AttachTo))

(event `/Game/VirtualRealityBP/Blueprints/PickupActorInterface.Drop`
  ;[0.402 0.7758 1] Calls parent BP_Pickup_Cube Drop functionality
  (`parent.Drop`))

(fn `UserConstructionScript`
  (`parent.UserConstructionScript`))