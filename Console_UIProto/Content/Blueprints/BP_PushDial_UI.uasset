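; BP_PushDial_UI is a grabbable dial control, derived from BP_Pickup_Cube, that turns with the grabbing hand and shows a dial widget while held.
; Each tick while held, hand relative roll drives DialObject, whose DialRoll feeds the UIW_Dial widget, and the mesh faces the player camera.
; The mesh is hidden at start, and dropping stops rotation, hides the widget, disables physics and restores the starting transform.
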(event `self.ReceiveBeginPlay`
  (`parent.ReceiveBeginPlay`)
  (set `self.startLocation` (`SceneComponent.K2_GetComponentToWorld` (`self.StaticMeshComponent`)))
  (`SceneComponent.SetVisibility` (`self.StaticMeshComponent`) false true))

(event `self.ReceiveTick`
  (params (DeltaSeconds :type "Float (single-precision)"))
  (bind _grabbinghand (`self.grabbingHand`))
  (bind _staticmeshcomponent (`self.StaticMeshComponent`))
  (bind _relativerotation_roll (`KismetMathLibrary.BreakRotator` (`SceneComponent.RelativeRotation` _grabbinghand)))
  (`parent.ReceiveTick` DeltaSeconds)
  (if (`KismetSystemLibrary.IsValid` _grabbinghand)
    (`/Game/Blueprints/BP_Dial_Object.Rotate Dial` (`self.dial_Object`) _relativerotation_roll)
    (`SceneComponent.K2_SetWorldRotation` _staticmeshcomponent (`KismetMathLibrary.FindLookAtRotation` (`SceneComponent.K2_GetComponentLocation` _staticmeshcomponent) (`PlayerCameraManager.GetCameraLocation` (`GameplayStatics.GetPlayerCameraManager` 0))) false false)
    (bind _asuiw_dial (cast `/Game/UIAssets/UIW_Dial` (`WidgetComponent.GetUserWidgetObject` (`self.dialUIW`))))
    (`/Game/UIAssets/UIW_Dial.Event TickerRotation` _asuiw_dial (`/Game/Blueprints/BP_Dial_Object.dialRoll` (`self.dial_Object`)))))

(event `self.Pickup`
  (params (AttachTo :type "SceneComponent Object Reference"))
  ;[0.402 0.7758 1] Calls parent BP_Pickup_Cube Pickup functionality
  (`parent.Pickup` AttachTo)
  (bind _output_get (set `self.grabbingHand` AttachTo))
  (bind _relativerotation_roll (`KismetMathLibrary.BreakRotator` (`SceneComponent.RelativeRotation` _output_get)))
  (`/Game/Blueprints/BP_Dial_Object.Start Dial Rotation` (`self.dial_Object`) _relativerotation_roll)
  (`SceneComponent.SetVisibility` (`self.dialUIW`) true false))

(event `self.Drop`
  ;[0.402 0.7758 1] Calls parent BP_Pickup_Cube Drop functionality
  (`parent.Drop`)
  (`PrimitiveComponent.SetSimulatePhysics` (`self.StaticMeshComponent`) false)
  (`/Game/Blueprints/BP_Dial_Object.Stop Dial Rotation` (`self.dial_Object`))
  (set `self.grabbingHand` null)
  (`SceneComponent.SetVisibility` (`self.dialUIW`) false false)
  (`SceneComponent.K2_SetWorldTransform` (`self.StaticMeshComponent`) (`self.startLocation`) false false))

(fn `UserConstructionScript`
  (`parent.UserConstructionScript`))