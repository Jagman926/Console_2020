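; PushDial is a VR dial actor that a motion controller grabs and turns by rolling the hand.
; Pickup records starting rolls, then Tick applies the hand's roll delta to the actor, wrapped to 0-360 degrees by RadialClamp.
; The angle feeds the UIW_Dial widget each frame, while HoldObject rides on the hand facing the camera.
; Drop detaches HoldObject and returns it to its BeginPlay transform.
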(event `self.ReceiveBeginPlay`
  (bind _holdobject (`self.holdObject`))
  (set `self.holdObjectStartLoc` (`SceneComponent.K2_GetComponentLocation` _holdobject))
  (set `self.holdObjectStartRot` (`SceneComponent.K2_GetComponentRotation` _holdobject))
  (`SceneComponent.SetVisibility` (`self.dialUIW`) true false))

(event `self.ReceiveTick`
  (params (DeltaSeconds :type "Float (single-precision)"))
  (bind _holdobject (`self.holdObject`))
  (if (`KismetSystemLibrary.IsValid` (`self.interactingHand`))
    (bind _out (`self.RadialClamp` (- (+ (.roll (`SceneComponent.RelativeRotation` (`self.interactingHand`))) (`self.baseRotation`)) (`self.startRotation`))))
    (bind _output_get (set `self.endRotation` _out))
    (`self.K2_SetActorRotation` (`KismetMathLibrary.MakeRotator` _output_get (.pitch (`self.K2_GetActorRotation` self)) (.yaw (`self.K2_GetActorRotation` self))))
    (`SceneComponent.K2_SetWorldRotation` _holdobject (`KismetMathLibrary.FindLookAtRotation` (`SceneComponent.K2_GetComponentLocation` _holdobject) (`PlayerCameraManager.GetCameraLocation` (`GameplayStatics.GetPlayerCameraManager` 0))) false false)
    (bind _asuiw_dial (cast `/Game/UIAssets/UIW_Dial` (`WidgetComponent.GetUserWidgetObject` (`self.dialUIW`))))
    (`/Game/UIAssets/UIW_Dial.Event TickerRotation` _asuiw_dial (`self.endRotation`))))

(event `/Game/VirtualRealityBP/Blueprints/PickupActorInterface.Pickup`
  (params (AttachTo :type "SceneComponent Object Reference"))
  (bind _output_get (set `self.interactingHand` AttachTo))
  (`SceneComponent.K2_AttachToComponent` (`self.holdObject`) _output_get "None" "KeepWorld" "KeepWorld" "KeepWorld" false)
  (set `self.baseRotation` (.roll (`self.K2_GetActorRotation` self)))
  (set `self.startRotation` (.roll (`SceneComponent.RelativeRotation` (`self.interactingHand`)))))

(event `/Game/VirtualRealityBP/Blueprints/PickupActorInterface.Drop`
  (`SceneComponent.K2_DetachFromComponent` (`self.holdObject`) "KeepWorld" "KeepWorld" "KeepWorld" false)
  (`SceneComponent.K2_SetWorldLocation` (`self.holdObject`) (`self.holdObjectStartLoc`) false false)
  (`SceneComponent.K2_SetWorldRotation` (`self.holdObject`) (`self.holdObjectStartRot`) false false)
  (set `self.interactingHand` null))

(fn `RadialClamp`
  (params (degree :type "Float (double-precision)"))
  (returns (out :type "Float (double-precision)"))
  (bind _returnvalue (mod degree 360.0))
  (if (< degree 0.0)
    (return (+ _returnvalue 360.0))
    (else
      (return _returnvalue))))

(fn `UserConstructionScript`
  (`parent.UserConstructionScript`))